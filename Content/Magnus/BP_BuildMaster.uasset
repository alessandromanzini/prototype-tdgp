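; BP_BuildMaster is an attacking building, likely a base for tower-style structures, that fires bullets at units within its range.
; Range enter and exit events maintain a Units list and call SelectTarget, which keeps the current EnemyTarget while listed, otherwise takes the first unit or clears it.
; A Tick countdown triggers Attack every AttackDelay, spawning a BP_Bullet at ProjSocket and passing it any valid target.
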(event Custom|Event%20Unit%20In%20Range
  (params (Unit :type Pawn%20Object%20Reference))
  (Utilities|Array|Add (Variables|Default|GetUnits) Unit)
  (CallFunction|SelectTarget))

(event Custom|Event%20Unit%20Out%20Of%20Range
  (params (Unit :type Pawn%20Object%20Reference))
  (Utilities|Array|RemoveItem (Variables|Default|GetUnits) Unit)
  (CallFunction|SelectTarget))

(event Custom|Event%20Attack
  (Utilities|IsValid (Variables|Default|GetEnemy%20Target)
    (:Is%20Valid
      (bind _returnvalue (Game|SpawnActorfromClass "/Game/Magnus/BP_Bullet.BP_Bullet_C" (Transformation|GetWorldTransform (Variables|Default|GetProjSocket)) "AdjustIfPossibleButAlwaysSpawn" "MultiplyWithRoot" 0 0))
      (Variables|/Game/Magnus/BP_Bullet.BP_Bullet_C|SetTarget _returnvalue (Variables|Default|GetEnemy%20Target)))))

(event EventBeginPlay)

(event Collision|EventActorBeginOverlap
  (params (OtherActor :type Actor%20Object%20Reference)))

(event EventTick
  (params (DeltaSeconds :type Float%20%28single-precision%29))
  (if (<= (Variables|Default|GetAttack%20Accumulated) 0.0)
    (Variables|Default|SetAttack%20Accumulated (Variables|Default|GetAttack%20Delay))
    (CallFunction|EventAttack)
    (else
      (Variables|Default|SetAttack%20Accumulated (- (Variables|Default|GetAttack%20Accumulated) DeltaSeconds)))))

(fn ConstructionScript)

(fn SelectTarget
  (bind _units (Variables|Default|GetUnits))
  (if (not (Utilities|Array|ContainsItem (Variables|Default|GetUnits) (Variables|Default|GetEnemy%20Target)))
    (if (Utilities|Array|IsEmpty _units)
      (Variables|Default|SetEnemy%20Target 0)
      (else
        (Variables|Default|SetEnemy%20Target (Utilities|Array|Get(acopy) _units))))))