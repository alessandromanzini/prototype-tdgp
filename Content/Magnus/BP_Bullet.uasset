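; BP_Bullet is a homing projectile that chases a single Target actor and damages it on contact.
; Each tick it offsets itself toward the Target's current location at ProjectileSpeed, without sweeping or any check that the Target is still valid.
; When Sphere1 overlaps the Target it applies ProjectileDamage and destroys itself, ignoring every other actor.
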(event OnComponentBeginOverlap(Sphere1)
  (params (OverlappedComponent :type Primitive%20Component%20Object%20Reference) (OtherActor :type Actor%20Object%20Reference) (OtherComp :type Primitive%20Component%20Object%20Reference) (OtherBodyIndex :type Integer) (bFromSweep :type Boolean) (SweepResult :type Hit%20Result%20Structure%20%28by%20ref%29))
  (bind _target (Variables|Default|GetTarget))
  (if (== OtherActor _target)
    (Game|Damage|ApplyDamage _target (Variables|Default|GetProjectile%20Damage) 0 0)
    (Actor|DestroyActor)))

(event EventBeginPlay)

(event Collision|EventActorBeginOverlap
  (params (OtherActor :type Actor%20Object%20Reference)))

(event EventTick
  (params (DeltaSeconds :type Float%20%28single-precision%29))
  (Transformation|AddActorWorldOffset (* (Math|Vector|Normalize (- (Transformation|GetActorLocation (Variables|Default|GetTarget)) (Transformation|GetActorLocation))) (* (Variables|Default|GetProjectile%20Speed) DeltaSeconds))))

(fn ConstructionScript)