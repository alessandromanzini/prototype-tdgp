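; Build-mode component for BP_CombatCharacter that previews and places buildings from the DT_Buildings data table.
; While build mode is toggled on, a per-tick camera line trace positions a collision-free preview mesh using M_BuildPreview.
; The mouse wheel changes the clamped build index and resets a DoOnce, so the preview is recreated with the new mesh.
; The apply input spawns the selected building's Blueprint at the preview transform.
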(event Custom|Preview%20Loop
  (bind _camera_ref (Variables|Default|GetCamera%20Ref))
  (bind _returnvalue (Transformation|GetWorldTransform _camera_ref))
  (bind (_outhit _returnvalue_2) (Collision|LineTraceByChannel (.location _returnvalue) (+ (.location _returnvalue) (* (Math|Vector|GetForwardVector (.rotation _returnvalue)) 1e+03)) "TraceTypeQuery1" false 0 "None"))
  (if _returnvalue_2
    (Utilities|FlowControl|Sequence
      (:then_0
        (Utilities|FlowControl|DoOnce false
          (:Completed
            (bind _returnvalue_3 (Game|AddComponentbyClass (Variables|Default|GetAs%20BP%20Combat%20Character) "/Script/Engine.StaticMeshComponent" false (Variables|Default|GetBuild%20Preview%20Transform)))
            (bind _output_get (Variables|Default|SetPreview%20Mesh _returnvalue_3))
            (Components|StaticMesh|SetStaticMesh _output_get (.mesh (Utilities|Array|Get(acopy) (Variables|Default|GetDT_Buildings) (Variables|Default|GetBuild%20Index))))
            (Rendering|Material|SetMaterial _output_get 0 "/Game/Magnus/Material/M_BuildPreview.M_BuildPreview")
            (Collision|SetCollisionEnabled _output_get "NoCollision"))))
      (:then_1
        (bind _output_get_2 (Variables|Default|SetBuild%20Preview%20Transform (Math|Transform|MakeTransform (.Location (Collision|BreakHitResult _outhit)) "0, 0, 0" "1.000000,1.000000,1.000000")))
        (Transformation|SetWorldTransform (Variables|Default|GetPreview%20Mesh) _output_get_2 false false)))))

(event Custom|Reset%20Build%20Mode
  (Utilities|FlowControl|DoOnce false) ; enters at Reset
)

(event Custom|Stop%20Build%20Mode
  (Variables|Default|SetinBuildMode false)
  (bind _preview_mesh (Variables|Default|GetPreview%20Mesh)
    (:then
      (Components|StaticMesh|SetStaticMesh _preview_mesh 0)
      (Variables|Default|SetPreview%20Mesh 0)
      (CallFunction|ResetBuildMode))
    (:else)))

(event Input|EnhancedActionEvents|EnhancedInputActionIA_Build
  (params (ActionValue :type Boolean) (ElapsedSeconds :type Float%20%28double-precision%29) (TriggeredSeconds :type Float%20%28double-precision%29) (InputAction :type Input%20Action%20Object%20Reference :default "/Game/Input/Actions/IA_Build.IA_Build"))
  (:Started
    (if (not (Variables|Default|GetinBuildMode))
      (Variables|Default|SetinBuildMode true)
      (else
        (Variables|Default|SetinBuildMode false)
        (bind _preview_mesh (Variables|Default|GetPreview%20Mesh)
          (:then
            (Components|StaticMesh|SetStaticMesh _preview_mesh 0)
            (Variables|Default|SetPreview%20Mesh 0)
            (CallFunction|ResetBuildMode))
          (:else))))))

(event Input|EnhancedActionEvents|EnhancedInputActionIA_ApplyBuild
  (params (ActionValue :type Boolean) (ElapsedSeconds :type Float%20%28double-precision%29) (TriggeredSeconds :type Float%20%28double-precision%29) (InputAction :type Input%20Action%20Object%20Reference :default "/Game/Input/Actions/IA_ApplyBuild.IA_ApplyBuild"))
  (:Started
    (if (Variables|Default|GetinBuildMode)
      (Game|SpawnActorfromClass (.blueprint (Utilities|Array|Get(acopy) (Variables|Default|GetDT_Buildings) (Variables|Default|GetBuild%20Index))) (Variables|Default|GetBuild%20Preview%20Transform) "Undefined" "MultiplyWithRoot" 0 0))))

(event EventBeginPlay
  (bind _asbp_combat_character (Utilities|Casting|CastToBP_CombatCharacter (Components|GetOwner)))
  (bind _output_get (Variables|Default|SetAs%20BP%20Combat%20Character _asbp_combat_character))
  (Variables|Default|SetCamera%20Ref (Variables|/Game/Variant_Combat/Blueprints/BP_CombatCharacter.BP_CombatCharacter_C|GetCamera _output_get))
  (bind _outrownames (DataTable|GetDataTableRowNames "/Game/Magnus/DT_Buildings.DT_Buildings"))
  (for _array_element _outrownames
    (bind _returnvalue (Utilities|GetDataTableRow "/Game/Magnus/DT_Buildings.DT_Buildings" _array_element)
      (:then
        (Utilities|Array|Add (Variables|Default|GetDT_Buildings) _returnvalue)))))

(event EventTick
  (params (DeltaSeconds :type Float%20%28single-precision%29))
  (if (Variables|Default|GetinBuildMode)
    (CallFunction|PreviewLoop)
    (Development|PrintString "BUILD MODE ACTIVE" true true "(R=0.000000,G=0.660000,B=1.000000,A=1.000000)" 0.005)))

(event Input|MouseEvents|MouseWheelUp
  (params (Key :type Key%20Structure :default "None"))
  (:Pressed
    (Variables|Default|SetBuild%20Index (Math|Integer|Clamp(Integer) (+ (Variables|Default|GetBuild%20Index) 1) 0 (- (Utilities|Array|Length (Variables|Default|GetDT_Buildings)) 1)))
    (bind _preview_mesh (Variables|Default|GetPreview%20Mesh)
      (:then
        (Components|StaticMesh|SetStaticMesh _preview_mesh 0)
        (Variables|Default|SetPreview%20Mesh 0)
        (CallFunction|ResetBuildMode))
      (:else))))

(event Input|MouseEvents|MouseWheelDown
  (params (Key :type Key%20Structure :default "None"))
  (:Pressed
    (Variables|Default|SetBuild%20Index (Math|Integer|Clamp(Integer) (- (Variables|Default|GetBuild%20Index) 1) 0 (- (Utilities|Array|Length (Variables|Default|GetDT_Buildings)) 1)))
    (bind _preview_mesh (Variables|Default|GetPreview%20Mesh)
      (:then
        (Components|StaticMesh|SetStaticMesh _preview_mesh 0)
        (Variables|Default|SetPreview%20Mesh 0)
        (CallFunction|ResetBuildMode))
      (:else))))